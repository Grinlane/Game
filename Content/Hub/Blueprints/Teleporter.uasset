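; Hub teleporter actor that opens a menu for picking a difficulty and travels to a random level from that difficulty's list.
; Any actor overlap creates the menu widget, shows the mouse cursor and switches input to UI only.
; Tick polls the button pressed states instead of binding click events; a difficulty button opens a level, while Exit removes the widget.
; Both paths hide the cursor and restore game-only input.
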(event EventBeginPlay)

(event Collision|EventActorBeginOverlap
  (params (OtherActor :type Actor%20Object%20Reference))
  (bind _returnvalue (Game|GetPlayerController 0))
  (Variables|/Script/Engine.PlayerController|SetbShowMouseCursor _returnvalue true)
  (Input|SetInputModeUIOnly _returnvalue 0 "DoNotLock" true)
  (bind _returnvalue_2 (UserInterface|CreateWidget "/Game/Blueprints/NewWidgetBlueprint.NewWidgetBlueprint_C" _returnvalue))
  (bind _returnvalue_3 (UserInterface|Viewport|AddtoPlayerScreen _returnvalue_2)))

(event EventTick
  (params (DeltaSeconds :type Float%20%28single-precision%29))
  (bind _returnvalue (Game|GetPlayerController 0))
  (bind _returnvalue_2 (Game|GetPlayerController 0))
  (bind _returnvalue_3 (Game|GetPlayerController 0))
  (if (stale Collision|EventActorBeginOverlap _returnvalue_3)
    (if (Class|Button|IsPressed (Variables|/Game/Blueprints/NewWidgetBlueprint.NewWidgetBlueprint_C|GetButton_Difficulty_1 (stale Collision|EventActorBeginOverlap _returnvalue_2)))
      (Variables|/Script/Engine.PlayerController|SetbShowMouseCursor _returnvalue_3 false)
      (Input|SetInputModeGameOnly _returnvalue_3 false)
      (Game|OpenLevel(byObjectReference) (.OutItem (Utilities|Array|Random (Variables|Default|GetDifficulty_1))))
      (elif (Class|Button|IsPressed (Variables|/Game/Blueprints/NewWidgetBlueprint.NewWidgetBlueprint_C|GetButton_Difficulty_2 (stale Collision|EventActorBeginOverlap _returnvalue_2)))
        (Variables|/Script/Engine.PlayerController|SetbShowMouseCursor _returnvalue false)
        (Input|SetInputModeGameOnly _returnvalue false)
        (Game|OpenLevel(byObjectReference) (.OutItem (Utilities|Array|Random (Variables|Default|GetDifficulty_2))))
        (elif (Class|Button|IsPressed (Variables|/Game/Blueprints/NewWidgetBlueprint.NewWidgetBlueprint_C|GetButton_Exit (stale Collision|EventActorBeginOverlap _returnvalue_2)))
          (Widget|RemovefromParent (stale Collision|EventActorBeginOverlap _returnvalue_2))
          (Variables|/Script/Engine.PlayerController|SetbShowMouseCursor _returnvalue_2 false)
          (Input|SetInputModeGameOnly _returnvalue_2 false))))))

(fn ConstructionScript)