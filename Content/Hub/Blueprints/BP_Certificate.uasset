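; BP_Certificate is a hub pickup actor that sells certificates to the player.
; When any actor overlaps it, it casts the game instance to GI_Main and, if money covers the fixed cost and the certificate count is below its maximum, deducts money and adds one certificate.
; Otherwise it prints a "NO MONEY" debug message, which also appears when the certificate cap is reached.
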(event EventBeginPlay)

(event Collision|EventActorBeginOverlap
  (params (OtherActor :type Actor%20Object%20Reference))
  (bind _asgi_main (Utilities|Casting|CastToGI_Main (Game|GetGameInstance)))
  (if (and (>= (Variables|/Game/GI_Main.GI_Main_C|GetMoney _asgi_main) 10) (< (Variables|/Game/GI_Main.GI_Main_C|GetCertificate _asgi_main) (Variables|/Game/GI_Main.GI_Main_C|GetCertificate%20Max _asgi_main)))
    (Variables|/Game/GI_Main.GI_Main_C|SetMoney _asgi_main (- (Variables|/Game/GI_Main.GI_Main_C|GetMoney _asgi_main) 10))
    (Variables|/Game/GI_Main.GI_Main_C|SetCertificate _asgi_main (+ (Variables|/Game/GI_Main.GI_Main_C|GetCertificate _asgi_main) 1))
    (else
      (Development|PrintString "NO MONEY"))))

(event EventTick
  (params (DeltaSeconds :type Float%20%28single-precision%29)))

(fn ConstructionScript)