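; Procedural dungeon generator that builds a level at BeginPlay from a random stream, seeded randomly or from the GameInstance.
; It starts at an entrance and recursively spawns rooms on random open exits, destroying any whose collision boxes overlap after a short delay.
; When the room budget or game-time limit is reached, it places special rooms, caps unused exits and adds loot meshes at random room loot spots.
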(event Custom|Spawn%20Entrance
  ;[1 1 1] Spawn Entrance
  (bind _returnvalue (Game|SpawnActorfromClass "/Game/Blueprints/Dungeon_Creator/Blockout_Assets/Rooms/CR_Entrance.CR_Entrance_C" (Transformation|GetWorldTransform (Variables|Default|GetDefaultSceneRoot)) "AlwaysSpawn" "MultiplyWithRoot" 0 0))
  (Utilities|Array|AppendArray (Variables|Default|GetExit%20List) (Components|GetChildrenComponents (Variables|/Game/Blueprints/Dungeon_Creator/Blockout_Assets/Rooms/CR_Entrance.CR_Entrance_C|GetExit%20Folder _returnvalue) false)))

(event Custom|Spawn%20Next
  (bind _seedstream (Variables|Default|GetSeedStream))
  ;[1 1 1] Spawn Next Room
  (if (Utilities|Array|IsNotEmpty (Variables|Default|GetExit%20List))
    (bind _output_get (Variables|Default|Setcurrent (.OutItem (Utilities|Array|RandomFromStream (Variables|Default|GetExit%20List) _seedstream))))
    (bind _aspossible_rooms (Utilities|Casting|CastToBP_NextRooms (Components|GetChildComponent _output_get 0)))
    (bind _returnvalue (Game|SpawnActorfromClass (.OutItem (Utilities|Array|RandomFromStream (Variables|/Game/Blueprints/Dungeon_Creator/BP_NextRooms.BP_NextRooms_C|GetpossibleRooms _aspossible_rooms) _seedstream)) (Transformation|GetWorldTransform (Variables|Default|Getcurrent)) "AlwaysSpawn" "MultiplyWithRoot" 0 0))
    (Variables|Default|SetLatest%20Room _returnvalue)
    (Utilities|FlowControl|Delay 0.001)
    (bind _overlapped (CallFunction|HandleOverlap))
    (if _overlapped
      _
      (else
        (Utilities|Array|RemoveItem (Variables|Default|GetExit%20List) (Variables|Default|Getcurrent))))
    (if (> (Variables|Default|GetRoomAmount) 0)
      (bind _newparam (CallFunction|CheckDungeonComplete))
      (if _newparam
        (CallFunction|SpawnSpecialRoom)
        (else
          (CallFunction|SpawnNext)))
      (else
        (CallFunction|SpawnSpecialRoom)))
    (else
      (CallFunction|CloseExits)
      (CallFunction|SpawnLoot))))

(event Custom|Add%20overlapping%20to%20List
  ;[1 1 1] Overlap List
  (for _array_element (Components|GetChildrenComponents (Variables|/Game/Blueprints/Dungeon_Creator/Master_Room.Master_Room_C|GetCollision (Variables|Default|GetLatest%20Room)) false)
    (bind _asbox_collision (Utilities|Casting|CastToBoxComponent _array_element))
    (Utilities|Array|AppendArray (Variables|Default|GetOverlappedList) (Class|PrimitiveComponent|GetOverlappingComponents _asbox_collision))))

(event Custom|SpawnLoot
  (bind _lootspots (Variables|Default|GetLootSpots))
  (bind _seedstream (Variables|Default|GetSeedStream))
  (bind _outitem (Utilities|Array|RandomFromStream _lootspots _seedstream))
  ;[1 1 1] Loot Spots
  (Development|PrintString "Hello")
  (bind _outactors (Actor|GetAllActorsOfClass "/Game/Blueprints/Dungeon_Creator/Master_Room.Master_Room_C"))
  (for _array_element _outactors
    (Utilities|Array|AppendArray (Variables|Default|GetLootSpots) (Components|GetChildrenComponents (Variables|/Game/Blueprints/Dungeon_Creator/Master_Room.Master_Room_C|GetLoot%20Folder _array_element) false)))
  (if (Utilities|Array|IsNotEmpty (Variables|Default|GetLootSpots))
    (for _index (range 0 (Variables|Default|GetLoot%20Amount))
      (AddComponent|AddStaticMeshComponent false (Transformation|GetWorldTransform _outitem))
      (Utilities|Array|RemoveItem (Variables|Default|GetLootSpots) _outitem))))

(event Custom|CloseExits
  ;[1 1 1] Close unused Exits
  (for _array_element (Variables|Default|GetExit%20List)
    (Game|SpawnActorfromClass (Variables|Default|GetExit_Mesh) (Transformation|GetWorldTransform _array_element) "Undefined" "MultiplyWithRoot" 0 0)))

(event Custom|SetSeed
  (bind _seedstream (Variables|Default|GetSeedStream))
  (bind _seedstream_2 (Variables|Default|GetSeedStream))
  ;[1 1 1] Set Seed
  (bind _asbp_game_instance (Utilities|Casting|CastToBP_GameInstance (Game|GetGameInstance)))
  (if (== (Variables|/Game/Blueprints/BP_GameInstance.BP_GameInstance_C|GetSeed _asbp_game_instance) -1)
    (Class|KismetMathLibrary|SeedRandomStream _seedstream_2)
    (bind _output_get (Variables|Default|SetCurrent%20Seed (Class|KismetMathLibrary|BreakRandomStream _seedstream_2)))
    (Development|PrintString (Utilities|String|ToString(Integer) _output_get))
    (else
      (bind _asbp_game_instance_2 (Utilities|Casting|CastToBP_GameInstance (Game|GetGameInstance)))
      (Math|Random|SetRandomStreamSeed _seedstream (Variables|/Game/Blueprints/BP_GameInstance.BP_GameInstance_C|GetSeed _asbp_game_instance_2))
      (bind _output_get_2 (Variables|Default|SetCurrent%20Seed (Class|KismetMathLibrary|BreakRandomStream _seedstream)))
      (Development|PrintString (Utilities|String|ToString(Integer) _output_get_2))
      (bind _asbp_game_instance_3 (Utilities|Casting|CastToBP_GameInstance (Game|GetGameInstance)))
      (Variables|/Game/Blueprints/BP_GameInstance.BP_GameInstance_C|SetSeed _asbp_game_instance_3 -1))))

(event Custom|Spawn%20Special%20Room
  (bind _seedstream (Variables|Default|GetSeedStream))
  ;[1 1 1] Spawn Special Room
  (if (Utilities|Array|IsNotEmpty (Variables|Default|GetSpecialRoomList))
    (bind _output_get (Variables|Default|SetSelectedSpecial (.OutItem (Utilities|Array|RandomFromStream (Variables|Default|GetSpecialRoomList) _seedstream))))
    (Variables|Default|Setcurrent (.OutItem (Utilities|Array|RandomFromStream (Variables|Default|GetExit%20List) _seedstream)))
    (bind _returnvalue (Game|SpawnActorfromClass _output_get (Transformation|GetWorldTransform (Variables|Default|Getcurrent)) "Undefined" "MultiplyWithRoot" 0 0))
    (bind _asmaster_room (Utilities|Casting|CastToMaster_Room _returnvalue))
    (Variables|Default|SetLatest%20Room _asmaster_room)
    (Utilities|FlowControl|Delay 0.001)
    (bind _overlapped (CallFunction|HandleOverlap))
    (if _overlapped
      (Utilities|Array|RemoveItem (Variables|Default|GetExit%20List) (Variables|Default|Getcurrent))
      (CallFunction|SpawnSpecialRoom)
      (else
        (Utilities|Array|RemoveItem (Variables|Default|GetExit%20List) (Variables|Default|Getcurrent))
        (Utilities|Array|RemoveItem (Variables|Default|GetSpecialRoomList) (Variables|Default|GetSelectedSpecial))
        (if (Utilities|Array|IsNotEmpty (Variables|Default|GetSpecialRoomList))
          (CallFunction|SpawnSpecialRoom)
          (else
            (CallFunction|CloseExits)
            (Development|PrintString "Dungeon Complete")
            (CallFunction|SpawnLoot)))))
    (else
      (CallFunction|CloseExits)
      (Development|PrintString "Dungeon Complete")
      (CallFunction|SpawnLoot))))

(event EventBeginPlay
  (CallFunction|SetSeed)
  (CallFunction|SpawnEntrance)
  (CallFunction|SpawnNext))

(fn ConstructionScript)

(fn HandleOverlap
  (CallFunction|AddOverlappingtoList)
  (if (Utilities|Array|IsNotEmpty (Variables|Default|GetOverlappedList))
    (Utilities|Array|Clear (Variables|Default|GetOverlappedList))
    (Actor|DestroyActor (Variables|Default|GetLatest%20Room))
    (return true)
    (else
      (Utilities|Array|Clear (Variables|Default|GetOverlappedList))
      (Variables|Default|SetRoomAmount (- (Variables|Default|GetRoomAmount) 1))
      (Utilities|Array|AppendArray (Variables|Default|GetExit%20List) (Components|GetChildrenComponents (Variables|/Game/Blueprints/Dungeon_Creator/Master_Room.Master_Room_C|GetExit%20Folder (Variables|Default|GetLatest%20Room)) false))
      (return false))))

(fn CheckDungeonComplete
  (bind _output_get (Variables|Default|SetMaxGenTime (Math|Conversions|ToFloat(Integer) (+ (Variables|Default|GetRoomAmount) 5))))
  (if (>= (Utilities|Time|GetGameTimeinSeconds) (+ _output_get 5.0))
    (return true)
    (else
      (return false))))